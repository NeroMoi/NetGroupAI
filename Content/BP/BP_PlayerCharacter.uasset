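; BP_PlayerCharacter is the player character Blueprint, which manages the in-game HUD and pause menu for the locally controlled player.
; On BeginPlay it sets game-only input, creates PlayerCharacterInfoHUD bound to itself, and broadcasts current health and energy.
; PauseGame opens PauseMenu with cursor and UI-only input, then pauses the game, which a comment marks as single-player only.
; EndPlay removes both widgets, and every path first checks for a local BP_GroupAIPlayerController.
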(event EventBeginPlay
  ;[1 1 1] 只使用本地控制器possess的PlayerCharacter
  (bind _asbp_group_aiplayer_controller (Utilities|Casting|CastToBP_GroupAIPlayerController (Pawn|GetController)))
  (if (Pawn|IsLocalController _asbp_group_aiplayer_controller)
    ;[1 1 1] 关闭光标，并将玩家的输入设为仅限游戏
    (Input|SetInputModeGameOnly _asbp_group_aiplayer_controller)
    ;[1 1 1] 将玩家的health和Energy信息通过PlayerCharacterInfoHUD输出
    (bind _returnvalue (UserInterface|CreateWidget "/Game/HUD/PlayerCharacterInfoHUD.PlayerCharacterInfoHUD_C"))
    (Variables|Default|SetCharacterInfoHUD _returnvalue)
    (Variables|/Game/HUD/PlayerCharacterInfoHUD.PlayerCharacterInfoHUD_C|SetPlayerCharacter (Variables|Default|GetCharacterInfoHUD) self)
    (Default|UpdateCharacterInfo (Variables|Default|GetCharacterInfoHUD))
    (Class|PlayerCharacter|BroadcastCurrentEnergy)
    (Class|PlayerCharacter|BroadcastCurrentHealth)
    (UserInterface|Viewport|AddtoViewport (Variables|Default|GetCharacterInfoHUD) 0)))

(event Collision|EventActorBeginOverlap
  (params (OtherActor :type Actor%20Object%20Reference)))

(event EventTick
  (params (DeltaSeconds :type Float%20%28single-precision%29)))

(event EventEndPlay
  (params (EndPlayReason :type EEndPlayReason%20Enum :default "Destroyed"))
  (bind _asbp_group_aiplayer_controller (Utilities|Casting|CastToBP_GroupAIPlayerController (Pawn|GetController)))
  (if (Pawn|IsLocalPlayerController _asbp_group_aiplayer_controller)
    (Widget|RemovefromParent (Variables|Default|GetCharacterInfoHUD))
    ;[1 1 1] 对应PauseHUD
    (Widget|RemovefromParent (Variables|Default|GetCurrentWidget))))

(event Input|ActionEvents|InputActionPauseGame
  (params (Key :type Key%20Structure))
  (bind _currentwidget (Variables|Default|GetCurrentWidget))
  (:Pressed
    (bind _asbp_group_aiplayer_controller (Utilities|Casting|CastToBP_GroupAIPlayerController (Pawn|GetController)))
    (if (Pawn|IsLocalPlayerController _asbp_group_aiplayer_controller)
      ;[1 1 1] 创建暂停菜单PauseMenu
      (Class|PlayerCharacter|ChangeMenuWidget "/Game/HUD/PauseMenu.PauseMenu_C")
      (Variables|/Script/Engine.PlayerController|SetbShowMouseCursor _asbp_group_aiplayer_controller true)
      (Input|SetInputModeUIOnly _asbp_group_aiplayer_controller _currentwidget "DoNotLock")
      (UserInterface|Viewport|AddtoViewport _currentwidget 0)
      ;[1 1 1] 只针对单机模式
      (Game|SetGamePaused true))))

(fn ConstructionScript)