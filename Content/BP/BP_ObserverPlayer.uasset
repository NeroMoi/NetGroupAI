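; BP_ObserverPlayer is an observer actor that shows information to the local player on cursor hover or overlap.
; Cursor hover finds the local BP_GroupAIPlayerController and toggles its HUD visibility.
; When an autonomous-proxy BP_PlayerCharacter overlaps, it creates or reuses a UserHUD filled with surplus pulls and shots.
; It also binds a debug name print to that character, which end overlap triggers before removing the widget.
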(event Custom|ShowObserverPlayerName
  (Development|PrintString (Utilities|String|Append "\"OverlapName:\"" (Variables|Default|GetSelfName)) true true "(R=0.000000,G=0.660000,B=1.000000,A=1.000000)" 5.0))

(event Custom|HideHUD
  (params (InController :type BP%20Group%20AI%20Player%20Controller%20Object%20Reference))
  (if (Pawn|IsLocalController InController)
    (Variables|/Script/Engine.HUD|SetbShowHUD (HUD|GetHUD InController) false)))

(event Custom|DisplayHUD
  (params (InController :type BP%20Group%20AI%20Player%20Controller%20Object%20Reference))
  (if (Pawn|IsLocalController InController)
    (Variables|/Script/Engine.HUD|SetbShowHUD (HUD|GetHUD InController) true)))

(event EventBeginPlay)

(event EventEndPlay
  (params (EndPlayReason :type EEndPlayReason%20Enum :default "Destroyed"))
  (switch Utilities|FlowControl|Switch|SwitchonEEndPlayReason EndPlayReason))

(event EventTick
  (params (DeltaSeconds :type Float%20%28single-precision%29)))

(event Collision|EventActorEndOverlap
  (params (OtherActor :type Actor%20Object%20Reference))
  (bind _asbp_player_character (Utilities|Casting|CastToBP_PlayerCharacter OtherActor))
  (if (Utilities|Enum|Equal(Enum) (Networking|GetLocalRole _asbp_player_character) "ROLE_AutonomousProxy")
    (Development|PrintString "\"end overlap\"")
    (Default|CallDisplayPlayerName _asbp_player_character)
    (Widget|RemovefromParent (Variables|Default|GetObserverWidgetHUD))))

(event MouseInput|EventActorBeginCursorOver
  (Development|PrintString "\"DisplayHUD\"")
  (bind _outactors (Actor|GetAllActorsOfClass "/Game/BP/BP_GroupAIPlayerController.BP_GroupAIPlayerController_C"))
  ;[1 1 1] 测试断点，查看server上响应的控制器的下标
  (bind (_array_element _array_index) (Utilities|Array|ForEachLoopwithBreak _outactors :!label _label)
    (:LoopBody
      (if (Pawn|IsLocalController _array_element)
        (Variables|Default|SetCurrentArrayIndex _array_index)
        (CallFunction|DisplayHUD _array_element)
        (goto _label Break)))))

(event MouseInput|EventActorEndCursorOver
  (Development|PrintString "\"HideHUD\"")
  (bind _outactors (Actor|GetAllActorsOfClass "/Game/BP/BP_GroupAIPlayerController.BP_GroupAIPlayerController_C"))
  (bind _array_element (Utilities|Array|ForEachLoopwithBreak _outactors :!label _label)
    (:LoopBody
      (if (Pawn|IsLocalController _array_element)
        (CallFunction|HideHUD _array_element)
        (goto _label Break)))))

(event Collision|EventActorBeginOverlap
  (params (OtherActor :type Actor%20Object%20Reference))
  (bind _observerwidgethud (Variables|Default|GetObserverWidgetHUD))
  (bind _asbp_player_character (Utilities|Casting|CastToBP_PlayerCharacter OtherActor))
  (if (Utilities|Enum|Equal(Enum) (Networking|GetLocalRole _asbp_player_character) "ROLE_AutonomousProxy")
    (EventDispatchers|BindEventtoDisplayPlayerName _asbp_player_character (delegate Custom|ShowObserverPlayerName))
    (Development|PrintString "\"Begin overlap\"")
    (if (== (Variables|Default|GetObserverWidgetHUD) 0)
      (bind _returnvalue (UserInterface|CreateWidget "/Game/HUD/UserHUD.UserHUD_C"))
      (|InitHUD _returnvalue _returnvalue _returnvalue _returnvalue)
      (else
        (|InitHUD_2 _observerwidgethud _observerwidgethud _observerwidgethud _observerwidgethud)))))

(fn ConstructionScript)